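; Elevator actor that travels between relative points, with a gate, and makes a further trip once the level is won.
; The construction script sets an InterpToMovement path from Location1 to Location2.
; Any actor overlap while BP_GameManager reports LevelWon rebuilds the path toward Location3, scales duration by Z ratio, and restarts movement with the gate visible and solid.
; When movement stops, the gate hides and loses collision.
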(event `self.ReceiveBeginPlay`
  (bind _returnvalue (`GameplayStatics.GetActorOfClass` "/Game/CustomContent/Blueprints/GameManagement/BP_GameManager.BP_GameManager_C"))
  (set `self.GMRef` _returnvalue))

(event `self.ReceiveActorBeginOverlap`
  (params (OtherActor :type "Actor Object Reference"))
  (bind _interptomovement (`self.InterpToMovement`))
  (bind _interptomovement_2 (`self.InterpToMovement`))
  (if (`/Game/CustomContent/Blueprints/GameManagement/BP_GameManager.Level Won` (`self.GMRef`))
    (`InterpToMovementComponent.ResetControlPoints` (`self.InterpToMovement`))
    (set `InterpToMovementComponent.ControlPoints` (`|MakeArray` (make `InterpControlPoint` (`self.Location1`)) (make `InterpControlPoint` (`self.Location3`))) _interptomovement)
    (set `InterpToMovementComponent.Duration` (* (`self.Duration`) (/ (.z (`self.Location3`)) (.z (`self.Location2`)))) _interptomovement)
    (`InterpToMovementComponent.FinaliseControlPoints` _interptomovement_2)
    (`InterpToMovementComponent.RestartMovement` _interptomovement_2 1.0)
    (`SceneComponent.SetVisibility` (`self.ElevatorGate`) true false)
    (`PrimitiveComponent.SetCollisionEnabled` (`self.ElevatorGate`) "QueryAndPhysics")))

(event `self.ReceiveTick`
  (params (DeltaSeconds :type "Float (single-precision)")))

(event `self.InterpToMovement.OnInterpToStop`
  (params (ImpactResult :type "HitResult Structure (by ref)") (Time :type "Float (single-precision)"))
  (`SceneComponent.SetVisibility` (`self.ElevatorGate`) false false)
  (`PrimitiveComponent.SetCollisionEnabled` (`self.ElevatorGate`) "NoCollision"))

(fn `UserConstructionScript`
  (bind _interptomovement (`self.InterpToMovement`))
  (set `InterpToMovementComponent.ControlPoints` (`|MakeArray` (make `InterpControlPoint` (`self.Location1`)) (make `InterpControlPoint` (`self.Location2`))) _interptomovement)
  (set `InterpToMovementComponent.Duration` (`self.Duration`) _interptomovement))