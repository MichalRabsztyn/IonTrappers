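; Bloch sphere actor that shows the state of one qubit as a 3D arrow.
; UpdateSphere copies Theta and Phi from the BP_GameManager qubit matching IonOnDisplayIndex.
; ValueChanged converts these angles to Cartesian coordinates, rotates the arrow with X negated and fires the EDValueChanged dispatcher.
; Text labels under the sphere are cached on BeginPlay and turned every tick using the look-at rotation from actor to camera.
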(event `self.ReceiveBeginPlay`
  (for _array_element (`SceneComponent.GetChildrenComponents` (`self.Sphere`) false)
    (bind _astext_render_component (cast `TextRenderComponent` _array_element))
    (`KismetArrayLibrary.Array_Add` (`self.Text Render Components`) _astext_render_component)
    (set `self.x` (* (`KismetMathLibrary.Sin` (`self.theta`)) (`KismetMathLibrary.Cos` (`self.phi`)) 50.0) :!label _label)
    (set `self.y` (* (`KismetMathLibrary.Sin` (`self.theta`)) (`KismetMathLibrary.Sin` (`self.phi`)) 50.0))
    (set `self.z` (* (`KismetMathLibrary.Cos` (`self.theta`)) 50.0))
    (`SceneComponent.K2_SetRelativeRotation` (`self.Arrow`) (`KismetMathLibrary.Conv_VectorToRotator` (`KismetMathLibrary.MakeVector` (* (`self.x`) -1.0) (`self.y`) (`self.z`))) false false)
    (`self.ED Value Changed`)))

(event `Value Changed`
  (goto _label))

(event `self.ReceiveTick`
  (params (DeltaSeconds :type "Float (single-precision)"))
  (for _array_element (`self.Text Render Components`)
    (`SceneComponent.K2_SetWorldRotation` _array_element (`KismetMathLibrary.FindLookAtRotation` (`self.K2_GetActorLocation`) (`self.K2_GetActorLocation` (`GameplayStatics.GetPlayerCameraManager` 0))) false false)))

(event `Update Sphere`
  (bind _returnvalue (`GameplayStatics.GetActorOfClass` "/Game/CustomContent/Blueprints/GameManagement/BP_GameManager.BP_GameManager_C"))
  (for (_array_element _array_index) (`/Game/CustomContent/Blueprints/GameManagement/BP_GameManager.Qubits` _returnvalue)
    (if (== _array_index (`self.Ion On Display Index`))
      (bind (_index _zeroprobability _oneprobability _theta _phi) (break `/Game/CustomContent/Blueprints/GameManagement/Qubit` _array_element))
      (set `self.theta` _theta)
      (set `self.phi` _phi)
      (`self.Value Changed`))))

(fn `UserConstructionScript`)