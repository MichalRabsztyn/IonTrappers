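; Actor that displays readouts for the 3D Bloch sphere: probabilities of |0> and |1> plus the theta and phi angles.
; On BeginPlay it finds the BP_BlochSphere3D actor, binds to its value-changed notification and puts a new W_BlochSphereInformation into its Widget component.
; Each change rewrites the actor's four text elements, deriving both probabilities linearly from the sphere's Z value and showing angles in radians.
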(event `self.ReceiveBeginPlay`
  (bind _returnvalue (`GameplayStatics.GetActorOfClass` "/Game/CustomContent/Blueprints/BlochSphere/BlochSphere3D/BP_BlochSphere3D.BP_BlochSphere3D_C"))
  (bind _output_get (set `self.Bloch Sphere 3D` _returnvalue))
  (add `/Game/CustomContent/Blueprints/BlochSphere/BlochSphere3D/BP_BlochSphere3D.ED Value Changed` _output_get (delegate `Show New Probability`))
  (bind _returnvalue_2 (`|CreateWidget` "/Game/CustomContent/Blueprints/BlochSphere/BlochSphere3D/W_BlochSphereInformation.W_BlochSphereInformation_C"))
  (`WidgetComponent.SetWidget` (`self.Widget`) _returnvalue_2))

(event `Show New Probability`
  (bind _bloch_sphere_3d (`self.Bloch Sphere 3D`))
  (bind _returnvalue (/ (- 50.0 (`/Game/CustomContent/Blueprints/BlochSphere/BlochSphere3D/BP_BlochSphere3D.z` (`self.Bloch Sphere 3D`))) 100.0))
  (`TextRenderComponent.K2_SetText` (`self.Prob0`) (`KismetTextLibrary.Conv_StringToText` (`KismetStringLibrary.Concat_StrStr` "Prob of |0>: " (`KismetStringLibrary.Conv_DoubleToString` (- 1.0 _returnvalue)))))
  (`TextRenderComponent.K2_SetText` (`self.Prob1`) (`KismetTextLibrary.Conv_StringToText` (`KismetStringLibrary.Concat_StrStr` "Prob of |1>: " (`KismetStringLibrary.Conv_DoubleToString` _returnvalue))))
  (`TextRenderComponent.K2_SetText` (`self.Theta:`) (`KismetTextLibrary.Conv_StringToText` (`KismetStringLibrary.Concat_StrStr` "Theta: " (`KismetStringLibrary.Conv_DoubleToString` (`/Game/CustomContent/Blueprints/BlochSphere/BlochSphere3D/BP_BlochSphere3D.theta` _bloch_sphere_3d)) " rad")))
  (`TextRenderComponent.K2_SetText` (`self.Phi:`) (`KismetTextLibrary.Conv_StringToText` (`KismetStringLibrary.Concat_StrStr` "Phi: " (`KismetStringLibrary.Conv_DoubleToString` (`/Game/CustomContent/Blueprints/BlochSphere/BlochSphere3D/BP_BlochSphere3D.phi` _bloch_sphere_3d)) " rad"))))

(fn `UserConstructionScript`)