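; BP_LevelChanger is a level-exit trigger that unlocks a level in the save file and loads a target level.
; Any overlap on its Cylinder component loads the "save1" slot, adds LevelToUnlockId uniquely to the BP_Save UnlockedLevels list, saves, then opens LevelToLoadName.
; The overlapping actor is not filtered.
; If no save exists, it only prints an error and the level does not change.
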(event `self.Cylinder.OnComponentBeginOverlap`
  (params (OverlappedComponent :type "PrimitiveComponent Object Reference") (OtherActor :type "Actor Object Reference") (OtherComp :type "PrimitiveComponent Object Reference") (OtherBodyIndex :type Integer) (bFromSweep :type Boolean) (SweepResult :type "HitResult Structure (by ref)"))
  (bind _returnvalue (`GameplayStatics.DoesSaveGameExist` "save1"))
  (if _returnvalue
    (bind _returnvalue_2 (`GameplayStatics.LoadGameFromSlot` "save1"))
    (bind _asbp_save (cast `/Game/CustomContent/Levels/Saves/BP_Save` _returnvalue_2))
    (`KismetArrayLibrary.Array_AddUnique` (`/Game/CustomContent/Levels/Saves/BP_Save.Unlocked Levels` _asbp_save) (`self.LevelToUnlockId`))
    (`GameplayStatics.SaveGameToSlot` _returnvalue_2 "save1")
    (`GameplayStatics.OpenLevel` (`self.LevelToLoadName`))
    (else
      (`KismetSystemLibrary.PrintString` "Failed to find save file"))))

(fn `UserConstructionScript`)