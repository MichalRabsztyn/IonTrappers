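; Game manager for an ion-qubit puzzle level, holding the qubit states and the win flag.
; BeginPlay initializes one qubit per ion in the zero state.
; Events pulse global lasers or fire local laser orders in sequence, timed from the gate data table.
; The win check passes if any qubit's one-probability is within margin of its target, and results visibility is randomly sampled from each one-probability, like a measurement.
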(event `self.ReceiveBeginPlay`
  (for _index (range (`self.Ion Count`))
    (`KismetArrayLibrary.Array_Add` (`self.Qubits`) (make `/Game/CustomContent/Blueprints/GameManagement/Qubit` _index))))

(event `LightGlobalLaser`
  (bind _returnvalue (`GameplayStatics.GetActorOfClass` "/Game/CustomContent/Blueprints/Lasers/Global/BP_GlobalLaserSpawner.BP_GlobalLaserSpawner_C"))
  (`/Game/CustomContent/Blueprints/Lasers/Global/BP_GlobalLaserSpawner.TurnOnGlobalLasers` _returnvalue)
  (`KismetSystemLibrary.Delay` 0.5)
  (`/Game/CustomContent/Blueprints/Lasers/Global/BP_GlobalLaserSpawner.TurnOffGlobalLasers` _returnvalue))

(event `LightLocalLasers`
  (params (`Laser Orders` :type "Array of /Game/CustomContent/Database/Struct_LaserOrders Structure"))
  (bind _returnvalue (`GameplayStatics.GetActorOfClass` "/Game/CustomContent/Blueprints/Lasers/Local/BP_LocalLaserSpawner.BP_LocalLaserSpawner_C"))
  (bind _index (`/Game/CustomContent/Macros/MacroLibrary.For Loop With Delay` 0 (- (`KismetArrayLibrary.Array_Length` `Laser Orders`) 1) (+ 0.5 (`.LaserShineDuration_26_F1DA829C4ACC781A054FFC93FD7C5896` (break `/Game/CustomContent/Database/Struct_GateDataset` (stale _returnvalue_2)))))
    (:`Loop Body`
      (bind _output (`|GetArrayItem` `Laser Orders` _index))
      (bind _returnvalue_2 (`|GetDataTableRow` "/Game/CustomContent/Database/Datatable_GatesDatabase.Datatable_GatesDatabase" (`KismetStringLibrary.Conv_StringToName` (`KismetStringLibrary.Conv_IntToString` (`.GateId_15_43638CEB42AEB0731E022EAA4B72FBFF` (break `/Game/CustomContent/Database/Struct_LaserOrders` _output)))))
        (:`then`
          (`/Game/CustomContent/Blueprints/Lasers/Local/BP_LocalLaserSpawner.TurnOnLocalLaser` _returnvalue _output))))))

(event `CheckWinConditions`
  (params (`Gates Left In Toolbox` :type Integer))
  (if true
    (for _array_element (`self.Qubits`)
      (bind (_index _zeroprobability _oneprobability) (break `/Game/CustomContent/Blueprints/GameManagement/Qubit` _array_element))
      (bind _output (`|GetArrayItem` (`self.Desired One Possibility Values For The Win`) _index))
      (if (and (>= _oneprobability (- _output (`self.Lower Possibility Value  Margin`))) (<= _oneprobability (+ _output (`self.Upper Possibility Value Margin`))))
        (set `self.Level Won` true)))))

(event `Show results`
  (bind _returnvalue (`GameplayStatics.GetActorOfClass` "/Game/CustomContent/Blueprints/Results/BP_ResultSpawner.BP_ResultSpawner_C"))
  (for (_array_element _array_index) (`/Game/CustomContent/Blueprints/Results/BP_ResultSpawner.ResultsRefs` _returnvalue)
    (if (>= (`.OneProbability_7_6DF069604DEF0DB513240182C6579D90` (break `/Game/CustomContent/Blueprints/GameManagement/Qubit` (`|GetArrayItem` (`self.Qubits`) _array_index))) (`KismetMathLibrary.RandomFloatInRange` 0.0 1.0))
      (bind _plane (`/Game/CustomContent/Blueprints/Results/BP_Result.Plane` _array_element))
      (`SceneComponent.SetVisibility` _plane true true)
      (else
        (`SceneComponent.SetVisibility` _plane false true)))))

(fn `UserConstructionScript`)