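; BP_ObjectSpawnManager sequences startup spawning of ions, local lasers, global lasers and results.
; InitializeObjectSpawner finds the four spawner actors, binds each one's completion callback to the next stage, then starts ion spawning.
; The last callback lets AFPController open its panel.
; InitializeScreenWidget populates MainScreenActor but sits outside this chain, and a laser turn-on loop is left disconnected.
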(event `self.ReceiveBeginPlay`)

(event `Initialize Object Spawner`
  (bind _returnvalue (`GameplayStatics.GetActorOfClass` "/Game/CustomContent/Blueprints/Ion/BP_IonSpawner.BP_IonSpawner_C"))
  (bind _output_get (set `self.IonSpawnerRef` _returnvalue))
  (add `/Game/CustomContent/Blueprints/Ion/BP_IonSpawner.IonSpawnerFinishedInitialization` _output_get (delegate `Initialize Local Laser Spawner`))
  (bind _returnvalue_2 (`GameplayStatics.GetActorOfClass` "/Game/CustomContent/Blueprints/Lasers/Local/BP_LocalLaserSpawner.BP_LocalLaserSpawner_C"))
  (bind _output_get_2 (set `self.LocalLaserSpawnerRef` _returnvalue_2))
  (add `/Game/CustomContent/Blueprints/Lasers/Local/BP_LocalLaserSpawner.LocalLaserSpawnerFinishedInitialization` _output_get_2 (delegate `Initialize Global Laser Spawner`))
  (bind _returnvalue_3 (`GameplayStatics.GetActorOfClass` "/Game/CustomContent/Blueprints/Lasers/Global/BP_GlobalLaserSpawner.BP_GlobalLaserSpawner_C"))
  (bind _output_get_3 (set `self.GlobalLaserSpawnerRef` _returnvalue_3))
  (add `/Game/CustomContent/Blueprints/Lasers/Global/BP_GlobalLaserSpawner.Global Laser Spawner Finished Initialization` _output_get_3 (delegate `Initialize Result Spawner`))
  (bind _returnvalue_4 (`GameplayStatics.GetActorOfClass` "/Game/CustomContent/Blueprints/Results/BP_ResultSpawner.BP_ResultSpawner_C"))
  (bind _output_get_4 (set `self.ResultsSpawnerRef` _returnvalue_4))
  (add `/Game/CustomContent/Blueprints/Results/BP_ResultSpawner.Result Spawner Finished Initialization` _output_get_4 (delegate `Initialize Character Panel`))
  (`self.Initialize Ion Spawner`))

(event `Initialize Ion Spawner`
  (`/Game/CustomContent/Blueprints/Ion/BP_IonSpawner.Spawn Ions` (`self.IonSpawnerRef`)))

(event `Initialize Local Laser Spawner`
  (`/Game/CustomContent/Blueprints/Lasers/Local/BP_LocalLaserSpawner.Spawn Local Lasers` (`self.LocalLaserSpawnerRef`)))

(event `Initialize Global Laser Spawner`
  (`/Game/CustomContent/Blueprints/Lasers/Global/BP_GlobalLaserSpawner.Spawn Global Lasers` (`self.GlobalLaserSpawnerRef`)))

(event `Initialize Result Spawner`
  (`/Game/CustomContent/Blueprints/Results/BP_ResultSpawner.Spawn Results` (`self.ResultsSpawnerRef`)))

(event `Initialize Screen Widget`
  (bind _returnvalue (`GameplayStatics.GetActorOfClass` "/Game/CustomContent/Blueprints/InteractiveScreen/MainScreenActor.MainScreenActor_C"))
  (`/Game/CustomContent/Blueprints/InteractiveScreen/MainScreenActor.PopulateScreenWidget` _returnvalue))

(event `Initialize Character Panel`
  (bind _returnvalue (`GameplayStatics.GetActorOfClass` "/Game/CustomContent/Character/AFPController.AFPController_C"))
  (set `/Game/CustomContent/Character/AFPController.bPanelCanBeOpened` true _returnvalue))

(fn `UserConstructionScript`)