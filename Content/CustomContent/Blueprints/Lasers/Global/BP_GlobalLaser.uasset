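; BP_GlobalLaser is an actor that draws a laser effect from its own position toward IonLocation.
; BeginPlay sets the Laser component's color to blue.
; Each Tick line-traces on the Camera channel toward IonLocation and feeds the hit point, or the target when nothing blocks, into the LaserEnd parameter, so blocking geometry cuts the beam short.
; An explicit Activate call on the Laser is present but never runs.
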(event `self.ReceiveBeginPlay`
  (`FXSystemComponent.SetColorParameter` (`self.Laser`) "Color" (struct :`G` 0.068602 :`B` 0.871367 :`A` 1.0)))

(event `self.ReceiveTick`
  (params (DeltaSeconds :type "Float (single-precision)"))
  (bind _returnvalue (`self.K2_GetActorLocation`))
  (bind _ion_location (`self.Ion Location`))
  (bind _returnvalue_2 (+ _returnvalue (* (`KismetMathLibrary.GetDirectionUnitVector` _returnvalue _ion_location) (`KismetMathLibrary.Vector_Distance` _returnvalue _ion_location))))
  (set `self.Trace End` _returnvalue_2)
  (bind _outhit (`KismetSystemLibrary.LineTraceSingle` _returnvalue _returnvalue_2 "TraceTypeQuery2"))
  (bind (_bblockinghit _binitialoverlap _time _distance _location) (`GameplayStatics.BreakHitResult` _outhit))
  (`FXSystemComponent.SetVectorParameter` (`self.Laser`) "LaserEnd" (select `bool` _bblockinghit :`false` (`self.Trace End`) :`true` _location)))

(fn `UserConstructionScript`)