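; BP_GlobalLaserSpawner spawns one BP_GlobalLaser per ion tracked by the game manager and toggles all global lasers on or off.
; SpawnGlobalLasers places each laser at the spawner's location and sets its IonLocation from that ion's position, with Z offset by the ion's Location1.
; It then caches every global laser in the level and signals that initialization is finished.
; Separate events activate or deactivate each cached laser's Laser component.
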(event `self.ReceiveBeginPlay`)

(event `Spawn Global Lasers`
  (bind _returnvalue (`GameplayStatics.GetActorOfClass` "/Game/CustomContent/Blueprints/GameManagement/BP_GameManager.BP_GameManager_C"))
  (bind _output_get (set `self.Ion Manager Ref` _returnvalue))
  (for _array_element (`/Game/CustomContent/Blueprints/GameManagement/BP_GameManager.Ions` _output_get)
    (bind _asbp_ion (cast `/Game/CustomContent/Blueprints/Ion/BP_Ion` _array_element))
    (bind _returnvalue_2 (`|SpawnActorFromClass` "/Game/CustomContent/Blueprints/Lasers/Global/BP_GlobalLaser.BP_GlobalLaser_C" (`KismetMathLibrary.Conv_VectorToTransform` (`self.K2_GetActorLocation`)) "Undefined" "OverrideRootScale" null null))
    (set `/Game/CustomContent/Blueprints/Lasers/Global/BP_GlobalLaser.Ion Location` (`KismetMathLibrary.MakeVector` (.x (`self.K2_GetActorLocation` _asbp_ion)) (.y (`self.K2_GetActorLocation` _asbp_ion)) (- (`KismetMathLibrary.Abs` (.z (`self.K2_GetActorLocation` _asbp_ion))) (.z (`/Game/CustomContent/Blueprints/Ion/BP_Ion.Location1` _asbp_ion)))) _returnvalue_2))
  (bind _outactors (`GameplayStatics.GetAllActorsOfClass` "/Game/CustomContent/Blueprints/Lasers/Global/BP_GlobalLaser.BP_GlobalLaser_C"))
  (set `self.GlobalLasers` _outactors)
  (`self.Global Laser Spawner Finished Initialization`))

(event `TurnOnGlobalLasers`
  (for _array_element (`self.GlobalLasers`)
    (`ActorComponent.Activate` (`/Game/CustomContent/Blueprints/Lasers/Global/BP_GlobalLaser.Laser` _array_element) false)))

(event `TurnOffGlobalLasers`
  (for _array_element (`self.GlobalLasers`)
    (`ActorComponent.Deactivate` (`/Game/CustomContent/Blueprints/Lasers/Global/BP_GlobalLaser.Laser` _array_element))))

(fn `UserConstructionScript`)