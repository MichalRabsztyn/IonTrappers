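; BP_LocalLaser is a laser beam actor that shines for a given duration.
; Each tick it traces on the Camera channel toward IonLocation, ending the green beam at the hit or maximum Distance.
; ShineLaser activates the beam and raises BP_GameManager's pending-order count until it finishes, while MainMenuShineLasers skips the count.
; MakeLaserofLength sets IonLocation as an offset from the actor and fixes the beam width.
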(event `self.ReceiveBeginPlay`
  (`FXSystemComponent.SetColorParameter` (`self.Laser`) "Color" (struct :`R` 0.003047 :`G` 0.826042 :`A` 1.0)))

(event `self.ReceiveTick`
  (params (DeltaSeconds :type "Float (single-precision)"))
  (bind _returnvalue (`self.K2_GetActorLocation`))
  (bind _returnvalue_2 (+ _returnvalue (* (`KismetMathLibrary.GetDirectionUnitVector` _returnvalue (`self.IonLocation`)) (`self.Distance`))))
  (set `self.TraceEnd` _returnvalue_2)
  (bind _outhit (`KismetSystemLibrary.LineTraceSingle` _returnvalue _returnvalue_2 "TraceTypeQuery2"))
  (bind (_bblockinghit _binitialoverlap _time _distance _location) (`GameplayStatics.BreakHitResult` _outhit))
  (`FXSystemComponent.SetVectorParameter` (`self.Laser`) "LaserEnd" (select `bool` _bblockinghit :`false` (`self.TraceEnd`) :`true` _location)))

(event `Shine Laser`
  (params (`Shine Duration` :type "Float (double-precision)"))
  (bind _returnvalue (`GameplayStatics.GetActorOfClass` "/Game/CustomContent/Blueprints/GameManagement/BP_GameManager.BP_GameManager_C"))
  (`ActorComponent.Activate` (`self.Laser`) false)
  (set `/Game/CustomContent/Blueprints/GameManagement/BP_GameManager.Pending Orders Count` (+ (`/Game/CustomContent/Blueprints/GameManagement/BP_GameManager.Pending Orders Count` _returnvalue) 1) _returnvalue)
  (`KismetSystemLibrary.Delay` `Shine Duration`)
  (`ActorComponent.Deactivate` (`self.Laser`))
  (bind _output_get (set `/Game/CustomContent/Blueprints/GameManagement/BP_GameManager.Pending Orders Count` (- (`/Game/CustomContent/Blueprints/GameManagement/BP_GameManager.Pending Orders Count` _returnvalue) 1) _returnvalue))
  (`KismetSystemLibrary.PrintString` (`KismetStringLibrary.Conv_IntToString` _output_get)))

(event `Make Laser of Length`
  (params (Length :type "Vector Structure"))
  (set `self.IonLocation` (+ Length (`self.K2_GetActorLocation`)))
  (`FXSystemComponent.SetFloatParameter` (`self.Laser`) "BeamWidth" 10.0))

(event `MainMenuShineLasers`
  (params (`Shine Duration` :type "Float (double-precision)"))
  (`ActorComponent.Activate` (`self.Laser`) false)
  (`KismetSystemLibrary.Delay` `Shine Duration`)
  (`ActorComponent.Deactivate` (`self.Laser`)))

(fn `UserConstructionScript`)