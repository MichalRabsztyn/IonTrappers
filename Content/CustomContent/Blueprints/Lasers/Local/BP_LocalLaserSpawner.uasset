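; Spawner that creates one local laser per ion and fires selected lasers for gate operations.
; SpawnLocalLasers reads the ions from BP_GameManager, spawns a BP_LocalLaser aligned to each ion's X on the spawner's Y/Z, then signals initialization is finished.
; TurnOnLocalLaser looks up the order's gate ID in the gates data table, then colors and shines the indexed lasers for that row's duration.
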(event `self.ReceiveBeginPlay`)

(event `Spawn Local Lasers`
  (bind _returnvalue (`GameplayStatics.GetActorOfClass` "/Game/CustomContent/Blueprints/GameManagement/BP_GameManager.BP_GameManager_C"))
  (bind _output_get (set `self.Ion Manager Ref` _returnvalue))
  (for _array_element (`/Game/CustomContent/Blueprints/GameManagement/BP_GameManager.Ions` _output_get)
    (bind _returnvalue_2 (`self.K2_GetActorLocation` _array_element))
    (bind _returnvalue_3 (`|SpawnActorFromClass` "/Game/CustomContent/Blueprints/Lasers/Local/BP_LocalLaser.BP_LocalLaser_C" (`KismetMathLibrary.Conv_VectorToTransform` (`KismetMathLibrary.MakeVector` (.x _returnvalue_2) (.y (`self.K2_GetActorLocation`)) (.z (`self.K2_GetActorLocation`)))) "Undefined" "OverrideRootScale" null null))
    (`FXSystemComponent.SetFloatParameter` (`/Game/CustomContent/Blueprints/Lasers/Local/BP_LocalLaser.Laser` _returnvalue_3) "BeamWidth" 50.0)
    (set `/Game/CustomContent/Blueprints/Lasers/Local/BP_LocalLaser.IonLocation` _returnvalue_2 _returnvalue_3)
    (`KismetArrayLibrary.Array_Add` (`self.LocalLasers`) _returnvalue_3))
  (`self.LocalLaserSpawnerFinishedInitialization`))

(event `TurnOnLocalLaser`
  (params (`Laser Orders` :type "/Game/CustomContent/Database/Struct_LaserOrders Structure"))
  (bind (_laserindex _gateid) (break `/Game/CustomContent/Database/Struct_LaserOrders` `Laser Orders`))
  (bind _returnvalue (`|GetDataTableRow` "/Game/CustomContent/Database/Datatable_GatesDatabase.Datatable_GatesDatabase" (`KismetStringLibrary.Conv_StringToName` (`KismetStringLibrary.Conv_IntToString` _gateid)))
    (:`then`
      (for _array_element _laserindex
        (bind _laser (`/Game/CustomContent/Blueprints/Lasers/Local/BP_LocalLaser.Laser` (`|GetArrayItem` (`self.LocalLasers`) _array_element)))
        (bind (_name _image _info _bhasparameter _parametervalue _parametername _lasershineduration _lasercolor) (break `/Game/CustomContent/Database/Struct_GateDataset` _returnvalue))
        (`FXSystemComponent.SetColorParameter` _laser "Color" (`KismetMathLibrary.Conv_ColorToLinearColor` _lasercolor))
        (bind _asbp_local_laser (cast `/Game/CustomContent/Blueprints/Lasers/Local/BP_LocalLaser` (`ActorComponent.GetOwner` _laser)))
        (`/Game/CustomContent/Blueprints/Lasers/Local/BP_LocalLaser.Shine Laser` _asbp_local_laser _lasershineduration)))))

(fn `ShineLasers`)

(fn `UserConstructionScript`)