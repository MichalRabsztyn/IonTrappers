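; BP_IonSpawner spawns an evenly spaced row of BP_Ion actors, configured by BP_GameManager.
; SpawnIons reads count, size and spacing to center the row on world X zero at the spawner's Y and Z, scaling each ion to size.
; Each ion receives its index, vertical movement endpoints and duration from the manager's amplitude and frequency.
; It then stores all ions on the manager and fires IonSpawnerFinishedInitialization.
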(event `self.ReceiveBeginPlay`)

(event `Spawn Ions`
  (bind _returnvalue (`GameplayStatics.GetActorOfClass` "/Game/CustomContent/Blueprints/GameManagement/BP_GameManager.BP_GameManager_C"))
  (bind _output_get (set `self.GameManagerRef` _returnvalue))
  (bind _asbp_game_manager (cast `/Game/CustomContent/Blueprints/GameManagement/BP_GameManager` _output_get))
  (bind _ion_count (`/Game/CustomContent/Blueprints/GameManagement/BP_GameManager.Ion Count` _asbp_game_manager))
  (for _index (range _ion_count)
    (bind _ion_size (`/Game/CustomContent/Blueprints/GameManagement/BP_GameManager.Ion Size` _asbp_game_manager))
    (bind _distance_between_ions (`/Game/CustomContent/Blueprints/GameManagement/BP_GameManager.Distance Between Ions` _asbp_game_manager))
    (bind _returnvalue_2 (/ (/ (`/Game/CustomContent/Blueprints/GameManagement/BP_GameManager.Ion Size` _asbp_game_manager) 2.0) 50.0))
    (bind _returnvalue_3 (/ (`/Game/CustomContent/Blueprints/GameManagement/BP_GameManager.Movement Amplitude` _asbp_game_manager) 2.0))
    (`|SpawnActorFromClass` "/Game/CustomContent/Blueprints/Ion/BP_Ion.BP_Ion_C" (`KismetMathLibrary.MakeTransform` (`KismetMathLibrary.MakeVector` (+ (- (* _ion_size 0.5) (/ (+ (* _ion_count _ion_size) (* (- _ion_count 1) _distance_between_ions)) 2.0)) (* _index (+ _ion_size _distance_between_ions))) (.y (`self.K2_GetActorLocation`)) (.z (`self.K2_GetActorLocation`))) (struct) (`KismetMathLibrary.MakeVector` _returnvalue_2 _returnvalue_2 _returnvalue_2)) "DontSpawnIfColliding" "OverrideRootScale" null (`KismetMathLibrary.MakeVector` 0.0 0.0 _returnvalue_3) (`KismetMathLibrary.MakeVector` 0.0 0.0 (* _returnvalue_3 -1.0)) (`/Game/CustomContent/Blueprints/GameManagement/BP_GameManager.Movement Frequency` _asbp_game_manager) (0.0 0.0 0.0) _index null))
  (bind _outactors (`GameplayStatics.GetAllActorsOfClass` "/Game/CustomContent/Blueprints/Ion/BP_Ion.BP_Ion_C"))
  (set `/Game/CustomContent/Blueprints/GameManagement/BP_GameManager.Ions` _outactors _asbp_game_manager)
  (`self.IonSpawnerFinishedInitialization`))

(fn `UserConstructionScript`)