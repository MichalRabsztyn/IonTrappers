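; BP_Ion is an ion actor that moves along an InterpToMovement path and can visually show superposition between stable and excited states.
; The construction script builds the path from two relative locations and a duration.
; BeginPlay creates emissive dynamic materials showing only the stable mesh.
; BeginSuperposition drives both opacities from a timeline that ping-pongs through a FlipFlop until EndSuperposition stops it and restores the stable look.
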(event `self.ReceiveBeginPlay`
  (bind _returnvalue (`PrimitiveComponent.CreateDynamicMaterialInstance` (`self.IonExcited`) 0 "/Game/CustomContent/Models/IonModel/Materials/EmissionPurple.EmissionPurple" "None"))
  (`MaterialInstanceDynamic.SetScalarParameterValue` _returnvalue "Opacity" 0.0)
  (bind _returnvalue_2 (`PrimitiveComponent.CreateDynamicMaterialInstance` (`self.IonStable`) 0 "/Game/CustomContent/Models/IonModel/Materials/EmissionPurple.EmissionPurple" "None"))
  (`MaterialInstanceDynamic.SetScalarParameterValue` _returnvalue_2 "Opacity" 1.0))

(event `Begin Superposition`
  (set `self.ShouldTimelineStop` false)
  (bind (_direction _opacity) (`Timeline|Timeline_0` :!via `PlayFromStart` :!label _label)
    (:`Update`
      (`MaterialInstanceDynamic.SetScalarParameterValue` (stale `self.ReceiveBeginPlay` _returnvalue) "Opacity" (- 1.0 (* _opacity 0.8)))
      (`MaterialInstanceDynamic.SetScalarParameterValue` (stale `self.ReceiveBeginPlay` _returnvalue_2) "Opacity" (* _opacity 0.2)))
    (:`Finished`
      (if (not (stale `End Superposition` _output_get))
        (`/Engine/EditorBlueprintResources/StandardMacros.FlipFlop`
          (:`A`
            (goto _label :!via `ReverseFromEnd`))
          (:`B`
            (goto _label :!via `PlayFromStart`)))))))

(event `End Superposition`
  (`MaterialInstanceDynamic.SetScalarParameterValue` (stale `self.ReceiveBeginPlay` _returnvalue) "Opacity" 0.0)
  (`MaterialInstanceDynamic.SetScalarParameterValue` (stale `self.ReceiveBeginPlay` _returnvalue_2) "Opacity" 1.0)
  (bind _output_get (set `self.ShouldTimelineStop` true))
  (goto _label :!via `Stop`))

(fn `UserConstructionScript`
  (bind _interptomovement (`self.InterpToMovement`))
  (set `InterpToMovementComponent.ControlPoints` (`|MakeArray` (make `InterpControlPoint` (`self.Location1`)) (make `InterpControlPoint` (`self.Location2`))) _interptomovement)
  (set `InterpToMovementComponent.Duration` (`self.Duration`) _interptomovement))