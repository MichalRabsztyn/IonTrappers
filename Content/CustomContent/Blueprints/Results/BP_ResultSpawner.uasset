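; BP_ResultSpawner spawns a centred row of BP_Result actors, one for each ion configured in BP_GameManager.
; SpawnResults derives their scale and X spacing from the manager's ion size and gap, both multiplied by DistanceScale.
; The row is centred on world X zero at the spawner's Y and Z, skipping colliding spawns.
; It then stores all BP_Result actors in ResultsArray and signals that initialization has finished.
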(event `self.ReceiveBeginPlay`)

(event `Spawn Results`
  (bind _distance_scale (`self.Distance Scale`))
  (bind _returnvalue (`GameplayStatics.GetActorOfClass` "/Game/CustomContent/Blueprints/GameManagement/BP_GameManager.BP_GameManager_C"))
  (bind _output_get (set `self.Ion Manager Ref` _returnvalue))
  (bind _ion_count (`/Game/CustomContent/Blueprints/GameManagement/BP_GameManager.Ion Count` _output_get))
  (for _index (range _ion_count)
    (bind _returnvalue_2 (* (`/Game/CustomContent/Blueprints/GameManagement/BP_GameManager.Ion Size` _output_get) _distance_scale))
    (bind _returnvalue_3 (* _distance_scale (`/Game/CustomContent/Blueprints/GameManagement/BP_GameManager.Distance Between Ions` _output_get)))
    (bind _returnvalue_4 (* (/ (/ (`/Game/CustomContent/Blueprints/GameManagement/BP_GameManager.Ion Size` _output_get) 2.0) 50.0) (`self.Distance Scale`)))
    (`|SpawnActorFromClass` "/Game/CustomContent/Blueprints/Results/BP_Result.BP_Result_C" (`KismetMathLibrary.MakeTransform` (`KismetMathLibrary.MakeVector` (+ (- (* _returnvalue_2 0.5) (/ (+ (* _ion_count _returnvalue_2) (* (- _ion_count 1) _returnvalue_3)) 2.0)) (* _index (+ _returnvalue_2 _returnvalue_3))) (.y (`self.K2_GetActorLocation`)) (.z (`self.K2_GetActorLocation`))) (struct) (`KismetMathLibrary.MakeVector` _returnvalue_4 _returnvalue_4 _returnvalue_4)) "DontSpawnIfColliding" "OverrideRootScale" null null))
  (bind _outactors (`GameplayStatics.GetAllActorsOfClass` "/Game/CustomContent/Blueprints/Results/BP_Result.BP_Result_C"))
  (set `self.ResultsArray` _outactors)
  (`self.Result Spawner Finished Initialization`))

(fn `UserConstructionScript`)