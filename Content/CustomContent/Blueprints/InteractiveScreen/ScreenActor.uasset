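; ScreenActor is an interactive in-world screen that displays a UMG widget through a WidgetComponent.
; TurnOnScreen creates a MainScreen widget, assigns it to the component, then finds the BP_ObjectSpawnManager in the level and initializes its object spawner.
; A separate PopulateScreenWidget event calls InitializeScreen on that widget.
; An older InteractiveScreenWidget version of the same logic remains but never runs.
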(event `self.ReceiveBeginPlay`)

(event `Turn On Screen`
  (bind _returnvalue (`|CreateWidget` "/Game/CustomContent/Blueprints/InteractiveScreen/MainScreen.MainScreen_C"))
  (bind _output_get (set `self.Main Screen Widget` _returnvalue))
  (`WidgetComponent.SetWidget` (`self.WidgetComponent`) _output_get)
  (bind _returnvalue_2 (`GameplayStatics.GetActorOfClass` "/Game/CustomContent/Blueprints/GameManagement/BP_ObjectSpawnManager.BP_ObjectSpawnManager_C"))
  (`/Game/CustomContent/Blueprints/GameManagement/BP_ObjectSpawnManager.Initialize Object Spawner` _returnvalue_2))

(event `PopulateScreenWidget`
  (`/Game/CustomContent/Blueprints/InteractiveScreen/MainScreen.Initialize Screen` (`self.Main Screen Widget`)))

(fn `UserConstructionScript`)